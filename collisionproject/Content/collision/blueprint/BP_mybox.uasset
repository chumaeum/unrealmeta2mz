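; BP_mybox is a trigger box, apparently for collision testing, that sets other actors in motion when something overlaps its Cube component.
; On begin overlap it calls Sphereevent on every Movesphere entry, then Play on every BPLeftright entry.
; Begin and end overlap print the component and actor names as long-lived debug messages.
; The hit event does nothing, and leftover loop and print nodes sit disconnected.
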(event OnComponentBeginOverlap(Cube)
  (params (OverlappedComponent :type Primitive%20Component%20Object%20Reference) (OtherActor :type Actor%20Object%20Reference) (OtherComp :type Primitive%20Component%20Object%20Reference) (OtherBodyIndex :type Integer) (bFromSweep :type Boolean) (SweepResult :type Hit%20Result%20Structure%20%28by%20ref%29))
  (Development|PrintString (Utilities|String|Append "overlapped compenent" (Utilities|GetDisplayName OverlappedComponent) "otheractor" (Utilities|GetDisplayName OtherActor) "othercomp" (Utilities|GetDisplayName OtherComp)) true true "(R=0.000000,G=0.660000,B=1.000000,A=1.000000)" 1e+02)
  (Utilities|FlowControl|Sequence
    (:then_0
      (for _array_element (Variables|Default|Getmovesphere)
        (Default|Sphereevent _array_element)))
    (:then_1
      (for _array_element_2 (Variables|Default|GetBP_leftright)
        (Default|Play _array_element_2)))))

(event OnComponentEndOverlap(Cube)
  (params (OverlappedComponent :type Primitive%20Component%20Object%20Reference) (OtherActor :type Actor%20Object%20Reference) (OtherComp :type Primitive%20Component%20Object%20Reference) (OtherBodyIndex :type Integer))
  (Development|PrintString (Utilities|String|Append "overlapped compenent" (Utilities|GetDisplayName OverlappedComponent) "otheractor" (Utilities|GetDisplayName OtherActor) "othercomp" (Utilities|GetDisplayName OtherComp)) true true "(R=0.000000,G=0.660000,B=1.000000,A=1.000000)" 1e+02))

(event OnComponentHit(Cube)
  (params (HitComponent :type Primitive%20Component%20Object%20Reference) (OtherActor :type Actor%20Object%20Reference) (OtherComp :type Primitive%20Component%20Object%20Reference) (NormalImpulse :type Vector :default "0, 0, 0") (Hit :type Hit%20Result%20Structure%20%28by%20ref%29)))

(event EventBeginPlay)

(fn ConstructionScript)