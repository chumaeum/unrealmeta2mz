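; Coin pickup actor that spins its Sphere mesh by a fixed step every Tick, without delta-time scaling.
; Any overlap on Sphere1 hides Sphere, turns off Sphere1's collision and prints a debug string through NewFunction0, then calls Coinend on the NewVar0 reference.
; The actor is never destroyed, and the near-duplicate 3coin function is only called from unwired nodes.
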(event OnComponentBeginOverlap(Sphere1)
  (params (OverlappedComponent :type Primitive%20Component%20Object%20Reference) (OtherActor :type Actor%20Object%20Reference) (OtherComp :type Primitive%20Component%20Object%20Reference) (OtherBodyIndex :type Integer) (bFromSweep :type Boolean) (SweepResult :type Hit%20Result%20Structure%20%28by%20ref%29))
  (CallFunction|NewFunction0)
  (Default|Coinend (Variables|Default|GetNewVar_0)))

(event EventTick
  (params (DeltaSeconds :type Float%20%28single-precision%29))
  (Transformation|AddWorldRotation (Variables|Default|GetSphere) "0,3.000000, 0" false false))

(fn ConstructionScript)

(fn 3coin
  (Rendering|SetVisibility (Variables|Default|GetSphere) false false)
  (Collision|SetCollisionEnabled (Variables|Default|GetSphere1) "NoCollision")
  (Development|PrintString "Hello"))

(fn NewFunction0
  (Rendering|SetVisibility (Variables|Default|GetSphere) false false)
  (Collision|SetCollisionEnabled (Variables|Default|GetSphere1) "NoCollision")
  (Development|PrintString "Hello"))