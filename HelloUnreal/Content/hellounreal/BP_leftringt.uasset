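; Test actor that slides its static mesh around by stepping its relative location.
; Tick runs UpdateMove, a back-and-forth X slide toggled by a bool, while a looping BeginPlay timer runs Move, an enum-driven square loop in X and Z, so both shift the same mesh.
; The delayed timer clear has an empty function name, so it does not target Move.
; R prints a debug string, but the input-enabling nodes are unconnected.
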(event Collision|EventActorBeginOverlap
  (params (OtherActor :type Actor%20Object%20Reference)))

(event EventBeginPlay
  (Utilities|Time|SetTimerbyFunctionName 0 "move" 0.01 true)
  (Utilities|FlowControl|Delay 0.2)
  (Utilities|Time|ClearTimerbyFunctionName 0 ""))

(event EventTick
  (params (DeltaSeconds :type Float%20%28single-precision%29))
  (CallFunction|UpdateMove))

(event Input|KeyboardEvents|R
  (params (Key :type Key%20Structure :default "None"))
  (:Pressed
    (Development|PrintString "Hello"))
  (:Released
    (Development|PrintString "Hello")))

(fn ConstructionScript)

(fn UpdateMove
  (bind _staticmesh (Variables|Default|GetStaticMesh))
  (if (Variables|Default|GetisMoveRight)
    (Transformation|AddRelativeLocation _staticmesh (Math|Vector|MakeVector 1e+01 0.0 0.0) false false)
    (if (> (.x (Variables|/Script/Engine.SceneComponent|GetRelativeLocation (Variables|Default|GetStaticMesh))) 1e+03)
      (Variables|Default|SetisMoveRight false))
    (else
      (Transformation|AddRelativeLocation _staticmesh "-10.000000, 0, 0" false false)
      (if (< (.x (Variables|/Script/Engine.SceneComponent|GetRelativeLocation (Variables|Default|GetStaticMesh))) 1e+01)
        (Variables|Default|SetisMoveRight true)))))

(fn Move
  (bind _staticmesh (Variables|Default|GetStaticMesh))
  (switch Utilities|FlowControl|Switch|SwitchonEn_movetype (Variables|Default|Getmovetype)
    (:NewEnumerator0
      (Transformation|AddRelativeLocation _staticmesh "10.000000, 0, 0" false false)
      (if (> (.x (Variables|/Script/Engine.SceneComponent|GetRelativeLocation (Variables|Default|GetStaticMesh))) 1e+02)
        (Variables|Default|Setmovetype "NewEnumerator1")))
    (:NewEnumerator1
      (Transformation|AddRelativeLocation _staticmesh "0,0.000000,10.000000" false false)
      (if (> (.z (Variables|/Script/Engine.SceneComponent|GetRelativeLocation (Variables|Default|GetStaticMesh))) 1e+02)
        (Variables|Default|Setmovetype "NewEnumerator2")))
    (:NewEnumerator2
      (Transformation|AddRelativeLocation _staticmesh "-10.000000, 0, 0" false false)
      (if (< (.x (Variables|/Script/Engine.SceneComponent|GetRelativeLocation (Variables|Default|GetStaticMesh))) 0.0)
        (Variables|Default|Setmovetype "NewEnumerator3")))
    (:NewEnumerator3
      (Transformation|AddRelativeLocation _staticmesh "0.000000, 0,-10.000000" false false)
      (if (< (.z (Variables|/Script/Engine.SceneComponent|GetRelativeLocation (Variables|Default|GetStaticMesh))) 0.0)
        (Variables|Default|Setmovetype "NewEnumerator0")))))