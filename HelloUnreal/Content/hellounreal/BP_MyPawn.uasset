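; BP_MyPawn is an experimental free-fly pawn with adjustable speed and debug prints.
; Move axes offset the actor along camera forward and right vectors, scaled by Speed without sweep or delta time; look axes drive controller pitch and yaw.
; SpeedUp effectively jumps to the clamp maximum, while SpeedDown steps down and prints.
; Time-formatting helpers, empty functions and disconnected nodes are leftover scratch work, with Tick doing nothing.
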(event EventTick
  (params (DeltaSeconds :type Float%20%28single-precision%29))
  ;[1 1 1] comment
)

(event Input|ActionEvents|InputActiontestkey
  (params (Key :type Key%20Structure :default "None"))
  (:Pressed
    (Development|PrintString "press"))
  (:Released
    (Development|PrintString "release")))

(event Input|ActionEvents|InputActionSpeedUp
  (params (Key :type Key%20Structure :default "None"))
  (:Pressed
    (Transformation|AddActorWorldOffset "0, 0, 0" (>= (+ (* 0 1) 10) 10))))

(event Input|ActionEvents|InputActionSpeedUp
  (params (Key :type Key%20Structure :default "None"))
  (:Pressed
    (bind _output_get (Variables|Default|Setspeed (Math|Float|Clamp(Float) (+ (Variables|Default|Getspeed) 101.0) 1e+01 1e+02)))))

(event Input|ActionEvents|InputActionSpeedDown
  (params (Key :type Key%20Structure :default "None"))
  (:Pressed
    (Variables|Default|Setspeed (Math|Float|Clamp(Float) (- (Variables|Default|Getspeed) 1.0) 1e+01 1e+02))
    (Development|PrintString (Utilities|String|ToString(Float) (Variables|Default|Getspeed)))))

(event Input|AxisEvents|InputAxisaxistest
  (params (AxisValue :type Float%20%28single-precision%29)))

(event Input|AxisEvents|InputAxisMoveFoward
  (params (AxisValue :type Float%20%28single-precision%29))
  (Transformation|AddActorWorldOffset (* (Transformation|GetActorForwardVector (Game|GetPlayerCameraManager 0)) (* AxisValue (Variables|Default|Getspeed)))))

(event Input|AxisEvents|InputAxisMoveRight
  (params (AxisValue :type Float%20%28single-precision%29))
  (Transformation|AddActorWorldOffset (* (Transformation|GetActorRightVector (Game|GetPlayerCameraManager 0)) (* AxisValue (Variables|Default|Getspeed)))))

(event Input|AxisEvents|InputAxisLookUp
  (params (AxisValue :type Float%20%28single-precision%29))
  (Pawn|Input|AddControllerPitchInput AxisValue))

(event Input|AxisEvents|InputAxisLookRight
  (params (AxisValue :type Float%20%28single-precision%29))
  (Pawn|Input|AddControllerYawInput AxisValue))

(event Input|KeyboardEvents|F
  (params (Key :type Key%20Structure :default "None")))

(fn ConstructionScript)

(fn Inttostr00
  (params (number :type Integer))
  (bind _returnvalue (Utilities|String|ToString(Integer) number))
  (if (< (Math|Conversions|ToFloat(Integer) number) 1e+01)
    (return (Utilities|String|Append "0" _returnvalue))
    (else
      (return _returnvalue))))

(fn NewFunction0)

(fn NewFunction1)

(fn Inttostr001
  (params (number :type Integer))
  (bind _returnvalue (Math|Conversions|ToFloat(Integer) number))
  (bind _returnvalue_2 (Math|Float|Floor _returnvalue))
  (bind _returnvalue_3 (Utilities|String|ToString(Integer) _returnvalue_2))
  (if (< (Math|Conversions|ToFloat(Integer) _returnvalue_2) 1e+01)
    (return (Utilities|String|Append "0" _returnvalue_3))
    (else
      (return _returnvalue_3))))

(fn PrintTime
  (params (delta%20second :type Float%20%28single-precision%29))
  (bind _output_get (Variables|Default|SetTotalDeltaSeconds (+ (Variables|Default|GetTotalDeltaSeconds) delta%20second)))
  (bind _string (CallFunction|Inttostr00 (Math|Float|Floor (/ 6e+01 _output_get))))
  (if true
    (Development|PrintString (Utilities|String|Append _string "분" "" "초"))))

(fn NewFunction2)

(fn NewFunction3
  (params (NewParam :type Integer))
  (if true
    (return "")
    (else
      (return ""))))